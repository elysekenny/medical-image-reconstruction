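; BP_GameController is a player-controlled camera rig that pans, zooms and rotates using Enhanced Input.
; Panning feeds movement input along the camera's right and forward vectors, flattened to the horizontal plane.
; Each tick lerps zoom and yaw rates toward their input values, driving a clamped spring arm length and the arm's rotation.
; Yaw updates only while rotation is allowed, which lasts until a short delay after the enabling input completes.
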(event `self.ReceiveTick`
  (params (DeltaSeconds :type "Float (single-precision)"))
  (`self.Adjust Camera Zoom`)
  (if (`self.Can Rotate`)
    (`self.Adjust Camera Rotation`)))

(event `EnhancedInput|/Game/Input/Actions/IA_AllowRotation`
  (params (ActionValue :type Boolean) (ElapsedSeconds :type "Float (double-precision)") (TriggeredSeconds :type "Float (double-precision)") (InputAction :type "InputAction Object Reference" :default "/Game/Input/Actions/IA_AllowRotation.IA_AllowRotation"))
  (:`Triggered`
    (set `self.Can Rotate` true))
  (:`Completed`
    (`KismetSystemLibrary.Delay` 0.5)
    (set `self.Can Rotate` false)))

(event `EnhancedInput|/Game/Input/Actions/IA_CameraMove`
  (params (ActionValue :type "Vector2D Structure") (ElapsedSeconds :type "Float (double-precision)") (TriggeredSeconds :type "Float (double-precision)") (InputAction :type "InputAction Object Reference" :default "/Game/Input/Actions/IA_CameraMove.IA_CameraMove"))
  (bind (_returnvalue_x _returnvalue_y) (`KismetMathLibrary.BreakVector` (`SceneComponent.GetRightVector` (`self.Camera`))))
  (bind (_returnvalue_x_2 _returnvalue_y_2) (`KismetMathLibrary.BreakVector` (`SceneComponent.GetForwardVector` (`self.Camera`))))
  (:`Triggered`
    (`self.AddMovementInput` (* (`KismetMathLibrary.Normal` (`KismetMathLibrary.MakeVector` _returnvalue_x _returnvalue_y)) (1000.0 1000.0 1000.0)) (* ActionValue_X 1000.0))
    (`self.AddMovementInput` (* (`KismetMathLibrary.Normal` (`KismetMathLibrary.MakeVector` _returnvalue_x_2 _returnvalue_y_2)) (1000.0 1000.0 1000.0)) (* ActionValue_Y 1000.0))))

(fn `Adjust Camera Rotation`
  (locals (Direction :type Integer :default 1))
  (bind _returnvalue_x (`KismetMathLibrary.BreakVector2D` (`|GetInputActionValue`)))
  (bind _output_get (set `self.Rotation Rate` (`KismetMathLibrary.Lerp` (`self.Rotation Rate`) _returnvalue_x (* (`GameplayStatics.GetWorldDeltaSeconds`) 24.0))))
  (`SceneComponent.K2_AddRelativeRotation` (`self.SpringArm`) (`KismetMathLibrary.MakeRotator` 0.0 0.0 _output_get) false false))

(fn `Adjust Camera Zoom`
  (bind _springarm (`self.SpringArm`))
  (bind _output_get (set `self.Zoom Rate` (`KismetMathLibrary.Lerp` (`self.Zoom Rate`) (* (`|GetInputActionValue`) -100.0) (* (`GameplayStatics.GetWorldDeltaSeconds`) 10.0))))
  (set `SpringArmComponent.TargetArmLength` (`KismetMathLibrary.FClamp` (+ (`SpringArmComponent.TargetArmLength` _springarm) _output_get) 500.0 10000.0) _springarm))

(fn `UserConstructionScript`)