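; BP_Marker is a clickable marker that toggles between selected and deselected states.
; Clicked flips the Selected flag, swaps the Marker component's material and sends HighlightMarkerMessage to player controller 0, passing itself when selected and nothing when deselected.
; Deselect reuses the deselection branch to restore the basic material and send the empty message, but leaves the Selected flag unchanged.
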(event `Clicked`
  (bind _returnvalue (`GameplayStatics.GetPlayerController` 0))
  (bind _selected (`self.Selected`))
  (set `self.Selected` (not _selected))
  (if _selected
    (`PrimitiveComponent.SetMaterial` (`self.Marker`) 0 "/Game/Materials/MI_Selected.MI_Selected")
    (message `/Game/Interfaces/BPI_PlayerController.Highlight Marker` _returnvalue self)
    (else
      (`PrimitiveComponent.SetMaterial` (`self.Marker`) 0 "/Engine/BasicShapes/BasicShapeMaterial.BasicShapeMaterial" :!label _label)
      (message `/Game/Interfaces/BPI_PlayerController.Highlight Marker` _returnvalue null))))

(event `Deselect`
  (goto _label))

(fn `UserConstructionScript`)