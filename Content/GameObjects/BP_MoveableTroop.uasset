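; BP_MoveableTroop is a click-selectable troop that can be sent to a destination with AI movement.
; Clicking toggles its selection circle and registers or clears the troop on the player controller through RegisterCharacterMessage.
; While Focused, Tick moves the player's controlled pawn to a fixed offset from the troop, so the view follows it.
; Goto runs AIMoveTo and clears Focused when the move succeeds or fails.
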(event `self.ReceiveActorOnClicked`
  (params (ButtonPressed :type "Key Structure"))
  (bind _selected (`self.Selected`))
  (`KismetSystemLibrary.PrintString` "Hello")
  (set `self.Selected` (not _selected))
  (if _selected
    (`SceneComponent.SetHiddenInGame` (`self.Selection Circle`) false false)
    (message `/Game/Interfaces/BPI_PlayerController.Register Character` (`GameplayStatics.GetPlayerController` 0) self)
    (else
      (`SceneComponent.SetHiddenInGame` (`self.Selection Circle`) true false)
      (message `/Game/Interfaces/BPI_PlayerController.Register Character` (`GameplayStatics.GetPlayerController` 0) null))))

(event `/Game/Interfaces/BPI_CharacterMovement.GoTo`
  (params (Destination :type "Vector Structure"))
  (`|AIMoveTo` self Destination null
    (:`OnSuccess`
      _)
    (:`OnFail`
      _))
  (set `self.Focused` false))

(event `self.ReceiveTick`
  (params (DeltaSeconds :type "Float (single-precision)"))
  (if (`self.Focused`)
    (`self.K2_SetActorLocation` (`Controller.K2_GetPawn` (`GameplayStatics.GetPlayerController` 0)) (+ (`self.K2_GetActorLocation`) (-350.0 0.0 0.0)) false false)))

(fn `UserConstructionScript`)