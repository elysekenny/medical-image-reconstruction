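; Clickable bacteria object that can be selected and deselected, with its mesh set from bacteria data by Initialise.
; A click sends itself and its ID to the player controller, then after a short delay toggles selection and the SelectionMarker's visibility.
; Deselecting by click notifies the controller that nothing is selected.
; OnDeselect clears the state and hides the marker so only one bacteria stays selected at a time.
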(event `self.ReceiveActorOnClicked`
  (params (ButtonPressed :type "Key Structure"))
  (bind _bacteria_data_id (break `/Game/Data/Struct_BacteriaData` (`self.Bacteria Data`)))
  ; Toggle selection on click
  (message `/Game/Interfaces/BPI_PlayerController.Select Bacteria` (`GameplayStatics.GetPlayerController` 0) self _bacteria_data_id)
  (`KismetSystemLibrary.Delay` 0.1)
  (bind _output_get (set `self.IsSelected` (not (`self.IsSelected`))))
  (`SceneComponent.SetHiddenInGame` (`self.Selection marker`) (not _output_get) false)
  (if (not (`self.IsSelected`))
    (message `/Game/Interfaces/BPI_PlayerController.No Bacteria Selected` (`GameplayStatics.GetPlayerController` 0))))

(event `On Deselect`
  ; can only have ONE bacteria selected, so when another is selected ensure this one gets deselected
  (set `self.IsSelected` false)
  (`SceneComponent.SetHiddenInGame` (`self.Selection marker`) true false))

(event `self.Bacteria Mesh.OnClicked`
  (params (TouchedComponent :type "PrimitiveComponent Object Reference") (ButtonPressed :type "Key Structure")))

(fn `Initialise`
  (params (`Bacteria Data` :type "/Game/Data/Struct_BacteriaData Structure"))
  (bind _output_get (set `self.Bacteria Data` `Bacteria Data`))
  (`StaticMeshComponent.SetStaticMesh` (`self.Bacteria Mesh`) (`.ModelReference_8_519C66B34A6B13B2E94635AA6C7B268D` (break `/Game/Data/Struct_BacteriaData` _output_get))))

(fn `UserConstructionScript`)